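; NemoBP is the player-one 2D flipbook character, with side-to-side movement, jumping and a kick.
; P1 inputs drive movement along world X and Jump, while holding kick sets an IsKicking flag.
; Tick picks the flipbook each frame: the jump animation while falling takes priority, then kick, then the default Nemo animation.
; The kick is purely visual here, with no hit detection or damage.
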(event EventTick
  (params (DeltaSeconds :type Float%20%28single-precision%29))
  ;[1 1 1] Om han hoppar spela hopp anim eller kick
  (if (AI|Components|NavMovement|IsFalling (Variables|Character|GetCharacterMovement))
    (Sprite|SetFlipbook (Variables|Default|GetSprite) "/Game/Karaktärer/NemoJump_Flipbook.NemoJump_Flipbook")
    (else
      (Sprite|SetFlipbook (Variables|Default|GetSprite) "/Game/Karaktärer/RiktigaNemo_Flipbook.RiktigaNemo_Flipbook")
      (if (Variables|Default|GetIsKicking?)
        (Sprite|SetFlipbook (Variables|Default|GetSprite) "/Game/Karaktärer/Kick_Flipbook.Kick_Flipbook")
        (else
          (Sprite|SetFlipbook (Variables|Default|GetSprite) "/Game/Karaktärer/RiktigaNemo_Flipbook.RiktigaNemo_Flipbook"))))))

(event Input|ActionEvents|InputActionJumpP1
  (params (Key :type Key%20Structure :default "None"))
  ;[1 1 1] Hopp
  (:Pressed
    (Character|Jump))
  (:Released
    (Character|StopJumping)))

(event Input|ActionEvents|InputActionkickP1
  (params (Key :type Key%20Structure :default "None"))
  ;[1 1 1] Kick
  (:Pressed
    (Variables|Default|SetIsKicking? true))
  (:Released
    (Variables|Default|SetIsKicking? false)))

(event Input|AxisEvents|InputAxisMoveRightP1
  (params (AxisValue :type Float%20%28single-precision%29))
  ;[1 1 1] Movement
  (Pawn|Input|AddMovementInput "1.000000, 0, 0" AxisValue false))

(fn ConstructionScript)